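; Mod tools Blueprint that enables debug input actions while the simulation runs, adding map teleport and a ghost mode toggle.
; On simulation begin it registers its actions and clears the development-only flag on the debug actions, restoring that flag and unregistering those on end.
; Teleport moves the local character to the visible map's cursor position, snapped to terrain.
; Ghost mode disables pawn collision and switches movement to flying.
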(event Custom|OnDebugTeleport
  (params (InputAction :type Input%20Action%20Data%20Object%20Reference) (Player :type Loc%20Player%20Controller%20Object%20Reference))
  (if (Variables|/Script/Loc.InputActionData|GetbWasPressed InputAction)
    (bind _foundwidgets (Widget|GetAllWidgetsOfClass "/Script/Loc.MapWidgetBase" false))
    (for _array_element _foundwidgets
      (bind _aswbp_map (Utilities|Casting|CastToWBP_Map _array_element))
      (if (Widget|IsVisible _array_element)
        (CallFunction|Teleport _aswbp_map)))))

(event Custom|ToggleGhostMode
  (params (InputAction :type Input%20Action%20Data%20Object%20Reference) (Player :type Loc%20Player%20Controller%20Object%20Reference))
  (if (Variables|/Script/Loc.InputActionData|GetbWasPressed InputAction)
    (bind _output_get (Variables|Default|SetbGohstMode (not (Variables|Default|GetbGohstMode))))
    (CallFunction|SetGhostMode _output_get)))

(event EventOnSimulationBegin
  (params (bIsLoading :type Boolean))
  (bind _returnvalue (Subsystems|GetInputContextSubsystem))
  (bind _returnvalue_2 (Subsystems|GetInputContextSubsystem))
  (EventDispatchers|BindEventtoOnInputActionStateChanged (Variables|Default|GetDebugTeleportAction) (EventDispatchers|CreateEvent :!event Custom|OnDebugTeleport))
  (EventDispatchers|BindEventtoOnInputActionStateChanged (Variables|Default|GetDebugToggleGhost) (EventDispatchers|CreateEvent :!event Custom|ToggleGhostMode))
  (Class|InputContextSubsystem|RegisterInputAction _returnvalue (Variables|Default|GetDebugTeleportAction))
  (Class|InputContextSubsystem|RegisterInputAction _returnvalue (Variables|Default|GetDebugToggleGhost))
  (for _array_element (Variables|Default|GetDebugActions)
    (Variables|/Script/Loc.InputActionData|SetbDevelopmentOnly _array_element false)
    (if (not (Utilities|Array|ContainsItem (Variables|/Script/Loc.InputContextSubsystem|GetRegisteredInputActions _returnvalue_2) _array_element))
      (Class|InputContextSubsystem|RegisterInputAction _returnvalue_2 _array_element))))

(event EventOnSimulationEnd
  (params (Reason :type EDestructionReason%20Enum :default "None"))
  (EventDispatchers|UnbindEventfromOnInputActionStateChanged (Variables|Default|GetDebugTeleportAction) (EventDispatchers|CreateEvent :!event Custom|OnDebugTeleport))
  (EventDispatchers|UnbindEventfromOnInputActionStateChanged (Variables|Default|GetDebugToggleGhost) (EventDispatchers|CreateEvent :!event Custom|ToggleGhostMode))
  (for _array_element (Variables|Default|GetDebugActions)
    (Variables|/Script/Loc.InputActionData|SetbDevelopmentOnly _array_element true)
    (Utilities|Array|RemoveItem (Variables|/Script/Loc.InputContextSubsystem|GetRegisteredInputActions (Subsystems|GetInputContextSubsystem)) _array_element)))

(fn ConstructionScript)

(fn Teleport
  (params (Map :type WBP%20Map%20Object%20Reference))
  (bind _returnvalue (Class|WorldGenerator|GetWorldPositionfromNormalizedMapPosition (Variables|/Script/Loc.Grid|GetWorldGenerator (Class|LocStatics|GetGridInstance)) (Default|GetCursorLocationNormalizedonMap Map)))
  (bind _asloc_character (Utilities|Casting|CastToLocCharacter (Pawn|GetControlledPawn (Class|LocStatics|GetLocalLocPlayerController))))
  (Class|LocCharacter|TeleportCharacterto _asloc_character (Math|Conversions|ToVector(Float) _returnvalue) "0, 0, 0" true false))

(fn SetGhostMode
  (params (bGhost :type Boolean))
  (bind _returnvalue (Class|LocStatics|GetLocalLocPlayerController))
  (bind _returnvalue_2 (Pawn|GetControlledPawn _returnvalue))
  (Development|PrintString (Utilities|String|ToString(Boolean) bGhost))
  (Collision|SetActorEnableCollision _returnvalue_2 (not bGhost))
  (Pawn|Components|CharacterMovement|SetMovementMode (Actor|GetComponentbyClass _returnvalue_2 "/Script/Engine.CharacterMovementComponent") (select bGhost "MOVE_Flying" "MOVE_Walking") 0))