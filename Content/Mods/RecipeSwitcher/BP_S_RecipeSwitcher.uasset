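; Simulation blueprint for a recipe switcher that sets the recipe of a neighboring grid object from a logic input signal.
; On each signal change it finds the selectable-recipes component at a rotation-adjusted grid offset, printing debug strings.
; If that component matches TargetRecipeSelection, it picks the on or off recipe from the signal state.
; When the recipe differs, it clears the processor's input and output inventories before switching.
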(event Custom|OnSignalChanged
  (params (Input :type Logic%20Connection%20Simulation%20Component%20Object%20Reference))
  (CallFunction|UpdateRecipe))

(event EventOnSimulationBegin
  (params (bIsLoading :type Boolean))
  (|CallParentFunction bIsLoading)
  (EventDispatchers|BindEventtoOnSignalChanged (Variables|Default|GetLogicInputSimulation) (EventDispatchers|CreateEvent :!event Custom|OnSignalChanged)))

(event EventOnSimulationEnd
  (params (Reason :type EDestructionReason%20Enum :default "None"))
  (|CallParentFunction Reason)
  (EventDispatchers|UnbindEventfromOnSignalChanged (Variables|Default|GetLogicInputSimulation) (EventDispatchers|CreateEvent :!event Custom|OnSignalChanged)))

(fn ConstructionScript)

(fn GetSelectableRecipeComponentatTarget
  (bind _targetpositionoffset (Variables|Default|GetTargetPositionOffset))
  (bind _positionsimulationcomponent (Variables|Default|GetPositionSimulationComponent))
  (bind _positionsimulationcomponent_2 (Variables|Default|GetPositionSimulationComponent))
  (bind _returnvalue (Class|PositionSimulationComponent|GetGridPosition _positionsimulationcomponent))
  (bind _returnvalue_2 (Class|PositionSimulationComponent|GetRotation _positionsimulationcomponent_2))
  (bind _returnvalue_3 (Class|LocCoreStatics|MakeFixedInt _returnvalue_2))
  (bind _returnvalue_4 (Class|LocStatics|RotateGridPosition _targetpositionoffset _returnvalue_3))
  (bind _returnvalue_5 (+ _returnvalue _returnvalue_4))
  (bind _returnvalue_6 (Class|LocStatics|GetGridObjectwithComponentat "/Script/Loc.SelectableRecipesSimulationComponent" _returnvalue_5))
  (Development|PrintString (Utilities|String|ToString(Integer) _returnvalue_5))
  (Development|PrintString (Utilities|GetDisplayName _returnvalue_6))
  (bind _asselectable_recipes_simulation_component (Utilities|Casting|CastToSelectableRecipesSimulationComponent _returnvalue_6)
    (:then
      (return (Utilities|ResolveSoftReference _asselectable_recipes_simulation_component)))
    (:CastFailed
      (return 0))))

(fn UpdateRecipe
  (bind _logicinputsimulation (Variables|Default|GetLogicInputSimulation))
  (bind _targetrecipeoff (Variables|Default|GetTargetRecipeOff))
  (bind _targetrecipeon (Variables|Default|GetTargetRecipeOn))
  (bind _returnvalue (Class|LogicConnectionSimulationComponent|GetStateasBool _logicinputsimulation))
  (bind _returnvalue_2 (select _returnvalue _targetrecipeon _targetrecipeoff))
  (bind _output (CallFunction|GetSelectableRecipeComponentatTarget))
  (if (== _output (Variables|Default|GetTargetRecipeSelection))
    (if (Utilities|IsValidSoftObjectReference _output)
      (if (!= (Class|SelectableRecipesSimulationComponent|GetSelectedRecipe (Utilities|ResolveSoftReference _output)) _returnvalue_2)
        (Class|InventoryComponent|Clear (Variables|/Script/Loc.RecipeProcessorSimulationComponent|GetInputInventory (Actor|GetComponentbyClass (Components|GetOwner (Utilities|ResolveSoftReference _output)) "/Script/Loc.RecipeProcessorSimulationComponent")))
        (Class|InventoryComponent|Clear (Variables|/Script/Loc.RecipeProcessorSimulationComponent|GetOutputInventory (Actor|GetComponentbyClass (Components|GetOwner (Utilities|ResolveSoftReference _output)) "/Script/Loc.RecipeProcessorSimulationComponent")))
        (Class|SelectableRecipesSimulationComponent|SetRecipe (Utilities|ResolveSoftReference _output) _returnvalue_2)))))