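; BP_S_Command_RecipeSwitcher_Set is a simulation command in the RecipeSwitcher mod that configures a recipe switcher.
; When run, it calls its parent, then checks that both the target recipe selector and the target switcher are valid.
; It assigns the selector as the switcher's target, optionally overwrites the On and Off recipes according to the SetOn and SetOff flags, then calls UpdateRecipe on the switcher.
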(event EventOnRunCommand
  (params (SimulationManager :type Simulation%20Manager%20Object%20Reference) (bRunAsPrediction :type Boolean))
  (bind _targetrecipeswitcher (Variables|Default|GetTargetRecipeSwitcher))
  (|CallParentFunction SimulationManager bRunAsPrediction)
  (Utilities|IsValid (Variables|Default|GetTargetRecipeSelector)
    (:Is%20Valid
      (Utilities|IsValid _targetrecipeswitcher
        (:Is%20Valid
          (Variables|/Game/Mods/RecipeSwitcher/BP_S_RecipeSwitcher.BP_S_RecipeSwitcher_C|SetTargetRecipeSelection _targetrecipeswitcher (Utilities|ResolveSoftReference (Variables|Default|GetTargetRecipeSelector)))
          (Utilities|FlowControl|Sequence
            (:then_0
              (if (Variables|Default|GetbSetOn)
                (Variables|/Game/Mods/RecipeSwitcher/BP_S_RecipeSwitcher.BP_S_RecipeSwitcher_C|SetTargetRecipeOn (Variables|Default|GetTargetRecipeSwitcher) (Variables|Default|GetRecipeOn))))
            (:then_1
              (if (Variables|Default|GetbSetOff)
                (Variables|/Game/Mods/RecipeSwitcher/BP_S_RecipeSwitcher.BP_S_RecipeSwitcher_C|SetTargetRecipeOff (Variables|Default|GetTargetRecipeSwitcher) (Variables|Default|GetRecipeOff))))
            (:then_2
              (Default|UpdateRecipe (Variables|Default|GetTargetRecipeSwitcher)))))))))